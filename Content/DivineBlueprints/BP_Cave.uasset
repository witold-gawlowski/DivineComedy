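; BP_Cave builds a block-based cave at BeginPlay.
; It calls GenerateCave, whose body is not in this graph, then CreateCave unpacks the flat CaveArray into X/Y/Z indices.
; Each true entry spawns an attached 6SidedCube, on a grid centred on the actor in X and Y.
; Indestructible outer-wall helpers exist, but their call is disconnected and most of their logic never runs.
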(event `self.ReceiveBeginPlay`
  (`self.GenerateCave`)
  (`self.Create Cave`))

(fn `Create Cave`
  (locals (x :type Integer) (y :type Integer) (z :type Integer) (Origin :type "Vector Structure"))
  (bind _cavearray (`self.CaveArray`))
  (set `local.Origin` (- (`SceneComponent.K2_GetComponentLocation` (`self.DefaultSceneRoot`)) (* (`KismetMathLibrary.MakeVector` (`KismetMathLibrary.Conv_IntToDouble` (`self.NumBlocsX`)) (`KismetMathLibrary.Conv_IntToDouble` (`self.NumBlocsY`))) (/ (`self.BlockSize`) 2.0))))
  (`KismetSystemLibrary.PrintString` (`KismetStringLibrary.Conv_IntToString` (`KismetArrayLibrary.Array_Length` _cavearray)))
  (for (_array_element _array_index) _cavearray
    (if _array_element
      (`self.CreateBlock` (/ _array_index (* (`self.NumBlocsY`) (`self.NumBlocsZGen`))) (mod (/ _array_index (`self.NumBlocsZGen`)) (`self.NumBlocsY`)) (mod _array_index (`self.NumBlocsZGen`)) (`local.Origin`))))
  (set `self.Cave3DSize` (`KismetMathLibrary.MakeVector` (`KismetMathLibrary.Conv_IntToDouble` (`self.NumBlocsX`)) (`KismetMathLibrary.Conv_IntToDouble` (`self.NumBlocsY`)) (`KismetMathLibrary.Conv_IntToDouble` (`self.NumBlocsZGen`)))))

(fn `Create Wall`
  (params (Transform :type "Transform Structure"))
  (`|SpawnActorFromClass` "/Game/DivineBlueprints/IndestructableWall.IndestructableWall_C" (`KismetMathLibrary.MakeTransform` (+ (`self.K2_GetActorLocation`) (.location Transform)) (.rotation Transform) (.scale Transform)) "Undefined" "OverrideRootScale"))

(fn `CreateBlock`
  (params (x :type Integer) (y :type Integer) (z :type Integer) (Origin :type "Vector Structure"))
  (bind _result (`/Engine/EditorBlueprintResources/StandardMacros.NegateFloat` (`KismetMathLibrary.Conv_IntToDouble` z))
    (:`  `
      (bind _returnvalue (`|SpawnActorFromClass` "/Game/DivineBlueprints/CubesVariation/6SidedCube.6SidedCube_C" (`KismetMathLibrary.MakeTransform` (+ Origin (* (`KismetMathLibrary.MakeVector` (`KismetMathLibrary.Conv_IntToDouble` x) (`KismetMathLibrary.Conv_IntToDouble` y) _result) (`self.BlockSize`)))) "Undefined" "OverrideRootScale"))
      (`self.K2_AttachToActor` _returnvalue self "None" "KeepRelative" "KeepRelative" "KeepRelative" true))))

(fn `Generate outer walls`
  (locals (HalfSize :type "Vector Structure"))
  (bind _blocksize (`self.BlockSize`))
  (bind _cave3dsize (`self.Cave3DSize`))
  (bind _result (`/Engine/EditorBlueprintResources/StandardMacros.NegateFloat` (.z _cave3dsize))
    (:`  `
      (`self.Create Wall` (`KismetMathLibrary.MakeTransform` (`KismetMathLibrary.MakeVector` -50.0 -50.0 _result) (struct) (+ (`KismetMathLibrary.MakeVector` (/ (.x _cave3dsize) _blocksize) (/ (.y _cave3dsize) _blocksize) 1.0) (0.0 0.0 0.0)))))))

(fn `UserConstructionScript`)