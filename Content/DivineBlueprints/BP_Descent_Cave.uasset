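; BP_Descent_Cave is a procedural cave generator variant that shapes a stepped, sloping passage through a block grid.
; Its construction script trims NumBlocsX to a multiple of NumBlocsZGen before running the parent script, so steps divide evenly.
; GenerationImprovements rewrites every CaveArray cell, clearing a diagonal band that shifts along X with each Z level, its width scaled by DoorframeHeight, and setting all others true.
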(event `self.GenerationImprovements`
  (bind _cavearray (`self.CaveArray`))
  (set `self.StepSize` (/ (`self.NumBlocsX`) (`self.NumBlocsZGen`)))
  (for (_ _array_index) _cavearray
    (bind (_x _y _z) (`self.ConvertArrayIndex` _array_index))
    (bind _returnvalue (* _z (`self.StepSize`)))
    (`KismetArrayLibrary.Array_Set` _cavearray _array_index (or (>= (/ (- _x _returnvalue) (`self.Doorframe height`)) (`self.StepSize`)) (< _x _returnvalue)))))

(fn `UserConstructionScript`
  (bind _numblocsx (`self.NumBlocsX`))
  (bind _returnvalue (mod _numblocsx (`self.NumBlocsZGen`)))
  (`|ExecutionSequence`
    (:`then_0`
      (if (!= _returnvalue 0)
        (set `self.NumBlocsX` (- _numblocsx _returnvalue))))
    (:`then_1`
      (`parent.UserConstructionScript`))))